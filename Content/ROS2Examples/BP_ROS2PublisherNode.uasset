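; Example ROS 2 publisher Blueprint that publishes string messages from Unreal through a ROS2Node.
; BeginPlay initializes the node, binds TimerEvent as the loop publisher's delegate and registers that publisher.
; TimerEvent fills each message with the current time, a greeting and an incrementing count.
; Disconnected graph sections, which never run, show two alternatives: a manually triggered non-loop publisher and a custom RRROS2StringPublisher class.
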(event `self.ReceiveBeginPlay`
  (bind _publisher (`ROS2PublisherComponent.Publisher` (`self.ROS2LoopPublisher`)))
  (`ROS2NodeComponent.Init` (`self.ROS2Node`))
  ;[1 1 1] Loop Publisher
  (`ROS2Publisher.SetDelegates` _publisher (delegate `TimerEvent`))
  (`ROS2NodeComponent.AddPublisher` (`self.ROS2Node`) _publisher))

(event `TimerEvent`
  (params (InTopicMessage :type "ROS2GenericMsg Object Reference"))
  (bind _returnvalue (`KismetMathLibrary.Now`))
  (bind _count (`self.Count`))
  ;[1 1 1] Loop Publisher
  (`ROS2StrMsg.SetMsg` (cast `ROS2StrMsg` InTopicMessage :!pure true) (make `ROSStr` (`KismetStringLibrary.Concat_StrStr` (`KismetTextLibrary.Conv_TextToString` (`KismetTextLibrary.AsTimeZoneTime_DateTime` _returnvalue)) (`KismetStringLibrary.Conv_IntToString` (`KismetMathLibrary.GetMillisecond` _returnvalue)) "Hello from BP " (`KismetStringLibrary.Conv_IntToString` _count))))
  (`/Engine/EditorBlueprintResources/StandardMacros.IncrementInt` _count))

(fn `UserConstructionScript`)