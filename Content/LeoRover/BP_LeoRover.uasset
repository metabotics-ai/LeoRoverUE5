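; BP_LeoRover is a Leo Rover robot vehicle Blueprint with a rocker suspension and four-wheel skid-steer drive.
; The construction script sets SkidDrive as the move component, binds the front and rear wheel physics constraints on both rockers, and sets the perimeter.
; Every tick it rewrites the Body's world rotation with pitch forced to zero, keeping roll and yaw, so the chassis stays level fore and aft.
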(event `self.ReceiveTick`
  (params (DeltaSeconds :type "Float (single-precision)"))
  (bind _body (`self.Body`))
  (bind (_returnvalue_roll _returnvalue_pitch _returnvalue_yaw) (`KismetMathLibrary.BreakRotator` (`KismetMathLibrary.TransformRotation` (`SceneComponent.K2_GetComponentToWorld` _body))))
  (`SceneComponent.K2_SetWorldRotation` _body (`KismetMathLibrary.MakeRotator` _returnvalue_roll 0.0 _returnvalue_yaw) false false))

(fn `UserConstructionScript`
  (bind _skiddrive (`self.SkidDrive`))
  (`self.SetMoveComponent` _skiddrive)
  (`SkidDriveComponent.SetWheels` _skiddrive (`self.PC_RockerLeft_WheelFrontLeft`) (`self.PC_RockerRight_WheelFrontRight`) (`self.PC_RockerLeft_WheelRearLeft`) (`self.PC_RockerRight_WheelRearRight`))
  (`SkidDriveComponent.SetPerimeter` _skiddrive))